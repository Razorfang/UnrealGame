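; Square grid actor Blueprint that exercises tile creation, removal and re-adding on a small 3D grid.
; On BeginPlay it initializes the tiles, nullifies one and adds it back at the same coordinate, printing the space count after each step.
; The grid functions it calls are not defined in these graphs.
; The construction script only prints a greeting, and the overlap and tick events are disabled stubs.
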(event `self.ReceiveBeginPlay`
  (`self.InitTiles` 3 3 2)
  (`KismetSystemLibrary.PrintString` (`KismetStringLibrary.Conv_IntToString` (`self.GetNumSpaces`)))
  (`self.NullifyTile` 1)
  (`KismetSystemLibrary.PrintString` (`KismetStringLibrary.Conv_IntToString` (`self.GetNumSpaces`)))
  (`self.AddTile` 1)
  (`KismetSystemLibrary.PrintString` (`KismetStringLibrary.Conv_IntToString` (`self.GetNumSpaces`))))

(fn `UserConstructionScript`
  (`KismetSystemLibrary.PrintString` "Hello"))